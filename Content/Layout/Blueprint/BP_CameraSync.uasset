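; Camera sync utility that mirrors CameraA's cine camera settings onto CameraB, both in the construction script and every Tick.
; It copies focal length, aperture, filmback, lens, crop and focus settings, plus world transform when SyncTransform is set.
; DisableFocus selects between copying the focus method and disabling it, but its branches are inverted between the two graphs: true disables focus at construction, while false disables it on Tick.
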(event EventTick
  (params (DeltaSeconds :type Float%20%28single-precision%29))
  (bind _cameraa (Variables|Default|GetCameraA))
  (bind _camerab (Variables|Default|GetCameraB))
  (bind _returnvalue (Class|CineCameraActor|GetCineCameraComponent _cameraa))
  (bind _returnvalue_2 (Class|CineCameraActor|GetCineCameraComponent _camerab))
  (Variables|/Script/CinematicCamera.CineCameraComponent|SetCurrentFocalLength _returnvalue_2 (Variables|/Script/CinematicCamera.CineCameraComponent|GetCurrentFocalLength _returnvalue))
  (Variables|/Script/CinematicCamera.CineCameraComponent|SetCurrentAperture _returnvalue_2 (Variables|/Script/CinematicCamera.CineCameraComponent|GetCurrentAperture _returnvalue))
  (Variables|/Script/CinematicCamera.CineCameraComponent|SetFilmback _returnvalue_2 (Variables|/Script/CinematicCamera.CineCameraComponent|GetFilmback _returnvalue))
  (Variables|/Script/CinematicCamera.CineCameraComponent|SetLensSettings _returnvalue_2 (Variables|/Script/CinematicCamera.CineCameraComponent|GetLensSettings _returnvalue))
  (Variables|/Script/CinematicCamera.CineCameraComponent|SetCropSettings _returnvalue_2 (Variables|/Script/CinematicCamera.CineCameraComponent|GetCropSettings _returnvalue))
  (Utilities|FlowControl|Sequence
    (:then_0
      (if (Variables|Default|GetSyncTransform)
        (Transformation|SetWorldTransform _returnvalue_2 (Transformation|GetWorldTransform _returnvalue) true true)))
    (:then_1
      (if (Variables|Default|GetDisableFocus)
        (Variables|/Script/CinematicCamera.CineCameraComponent|SetFocusSettings _returnvalue_2 (Utilities|Struct|MakeCameraFocusSettings (.focusmethod (Variables|/Script/CinematicCamera.CineCameraComponent|GetFocusSettings _returnvalue)) (.manualfocusdistance (Variables|/Script/CinematicCamera.CineCameraComponent|GetFocusSettings _returnvalue)) (.trackingfocussettings (Variables|/Script/CinematicCamera.CineCameraComponent|GetFocusSettings _returnvalue)) (.bsmoothfocuschanges (Variables|/Script/CinematicCamera.CineCameraComponent|GetFocusSettings _returnvalue)) (.focussmoothinginterpspeed (Variables|/Script/CinematicCamera.CineCameraComponent|GetFocusSettings _returnvalue)) (.focusoffset (Variables|/Script/CinematicCamera.CineCameraComponent|GetFocusSettings _returnvalue))))
        (else
          (Variables|/Script/CinematicCamera.CineCameraComponent|SetFocusSettings _returnvalue_2 (Utilities|Struct|MakeCameraFocusSettings "Disable" (.manualfocusdistance (Variables|/Script/CinematicCamera.CineCameraComponent|GetFocusSettings _returnvalue_2)) (.trackingfocussettings (Variables|/Script/CinematicCamera.CineCameraComponent|GetFocusSettings _returnvalue)) (.bsmoothfocuschanges (Variables|/Script/CinematicCamera.CineCameraComponent|GetFocusSettings _returnvalue)) (.focussmoothinginterpspeed (Variables|/Script/CinematicCamera.CineCameraComponent|GetFocusSettings _returnvalue)) (.focusoffset (Variables|/Script/CinematicCamera.CineCameraComponent|GetFocusSettings _returnvalue)))))))))

(fn ConstructionScript
  (bind _cameraa (Variables|Default|GetCameraA))
  (bind _camerab (Variables|Default|GetCameraB))
  (bind _returnvalue (Class|CineCameraActor|GetCineCameraComponent _cameraa))
  (bind _returnvalue_2 (Class|CineCameraActor|GetCineCameraComponent _camerab))
  (Variables|/Script/CinematicCamera.CineCameraComponent|SetCurrentFocalLength _returnvalue_2 (Variables|/Script/CinematicCamera.CineCameraComponent|GetCurrentFocalLength _returnvalue))
  (Variables|/Script/CinematicCamera.CineCameraComponent|SetCurrentAperture _returnvalue_2 (Variables|/Script/CinematicCamera.CineCameraComponent|GetCurrentAperture _returnvalue))
  (Variables|/Script/CinematicCamera.CineCameraComponent|SetFilmback _returnvalue_2 (Variables|/Script/CinematicCamera.CineCameraComponent|GetFilmback _returnvalue))
  (Variables|/Script/CinematicCamera.CineCameraComponent|SetLensSettings _returnvalue_2 (Variables|/Script/CinematicCamera.CineCameraComponent|GetLensSettings _returnvalue))
  (Variables|/Script/CinematicCamera.CineCameraComponent|SetCropSettings _returnvalue_2 (Variables|/Script/CinematicCamera.CineCameraComponent|GetCropSettings _returnvalue))
  (Utilities|FlowControl|Sequence
    (:then_0
      (if (Variables|Default|GetSyncTransform)
        (Transformation|SetWorldTransform _returnvalue_2 (Transformation|GetWorldTransform _returnvalue) true true)))
    (:then_1
      (if (Variables|Default|GetDisableFocus)
        (Variables|/Script/CinematicCamera.CineCameraComponent|SetFocusSettings _returnvalue_2 (Utilities|Struct|MakeCameraFocusSettings "Disable" (.manualfocusdistance (Variables|/Script/CinematicCamera.CineCameraComponent|GetFocusSettings _returnvalue_2)) (.trackingfocussettings (Variables|/Script/CinematicCamera.CineCameraComponent|GetFocusSettings _returnvalue)) (.bsmoothfocuschanges (Variables|/Script/CinematicCamera.CineCameraComponent|GetFocusSettings _returnvalue)) (.focussmoothinginterpspeed (Variables|/Script/CinematicCamera.CineCameraComponent|GetFocusSettings _returnvalue)) (.focusoffset (Variables|/Script/CinematicCamera.CineCameraComponent|GetFocusSettings _returnvalue))))
        (else
          (Variables|/Script/CinematicCamera.CineCameraComponent|SetFocusSettings _returnvalue_2 (Utilities|Struct|MakeCameraFocusSettings (.focusmethod (Variables|/Script/CinematicCamera.CineCameraComponent|GetFocusSettings _returnvalue)) (.manualfocusdistance (Variables|/Script/CinematicCamera.CineCameraComponent|GetFocusSettings _returnvalue)) (.trackingfocussettings (Variables|/Script/CinematicCamera.CineCameraComponent|GetFocusSettings _returnvalue)) (.bsmoothfocuschanges (Variables|/Script/CinematicCamera.CineCameraComponent|GetFocusSettings _returnvalue)) (.focussmoothinginterpspeed (Variables|/Script/CinematicCamera.CineCameraComponent|GetFocusSettings _returnvalue)) (.focusoffset (Variables|/Script/CinematicCamera.CineCameraComponent|GetFocusSettings _returnvalue)))))))))